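; Lobby game mode that gathers players in a multiplayer session and starts the match on Arena_map.
; On login it compares the player count to the session's connection count, server travelling after a short retriggerable delay when full and kicking extra players.
; It tracks lobby controllers, removing them on logout, and relays each join through them to print the player's name, noted as broken for clients.
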(event Custom|CE_tell_join_lobby_to_all
  (params (Player_name :type String))
  ;[1 0 0] ne marche pas pour les clients
  ;;[1 1 1] tells everyone a new player joined the lobby
  (for _array_element (Variables|Default|Getplayer_controllers)
    (bind _aspc_lobby (Utilities|Casting|CastToPC_lobby _array_element))
    (Default|CEPrintJoiningPlayerName _aspc_lobby Player_name)))

(event EventPostLogin
  (params (NewPlayer :type Player%20Controller%20Object%20Reference))
  (bind _returnvalue (Game|GetGameState))
  (bind _playername (Class|AdvancedSessionsLibrary|GetPlayerName NewPlayer))
  (bind _playerarray (Variables|/Script/Engine.GameStateBase|GetPlayerArray _returnvalue))
  (bind _returnvalue_2 (Utilities|Array|Length _playerarray))
  ;[1 1 1] lance la partie et kick les joueurs en trop
  (bind (_numconnections _numprivateconnections _bislan _bisdedicated _ballowinvites _ballowjoininprogress _bisanticheatenabled _builduniqueid _extrasettings) (Class|AdvancedSessionsLibrary|GetSessionSettings)
    (:OnSuccess
      (if (== _numconnections _returnvalue_2)
        (Utilities|Array|AddUnique (Variables|Default|Getplayer_controllers) NewPlayer)
        (CallFunction|CETellJoinLobbytoAll _playername)
        (Utilities|FlowControl|RetriggerableDelay 3.0)
        (Development|ExecuteConsoleCommand "serverTravel Arena_map" 0)
        (elif (> _numconnections _returnvalue_2)
          (Utilities|Array|AddUnique (Variables|Default|Getplayer_controllers) 0)
          (CallFunction|CETellJoinLobbytoAll _playername)
          (else
            (Class|AdvancedSessionsLibrary|KickPlayer NewPlayer "too many players")
            (|UpdateSession _extrasettings _numconnections 0 false false false true false)))))))

(event EventOnLogout
  (params (ExitingController :type Controller%20Object%20Reference))
  ;[1 1 1] logout
  (bind _aspc_lobby (Utilities|Casting|CastToPC_lobby ExitingController))
  (Utilities|Array|RemoveItem (Variables|Default|Getplayer_controllers) _aspc_lobby))

(fn ConstructionScript)