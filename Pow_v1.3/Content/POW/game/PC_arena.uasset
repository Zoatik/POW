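; Player controller for the turn-based card arena: builds the HUD, animates the opening hand and relays turn changes.
; On their turn, players drop troop cards, validated client and server side before spawning, and click to select, move or attack.
; Off turn, clicks go to grid cells.
; Terrain edits queue in PS_arena, with server calls only from remote clients to avoid double application; also handles pause, notifications and debug keys.
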(event Custom|CE_C_end_turn
  ;[1 1 1] turn system
  (CallFunction|SetMyTurn false))

(event Custom|CE_C_start_turn
  ;[1 1 1] turn system
  (CallFunction|SetMyTurn true))

(event Custom|CE_handle_card_drop
  (params (card_infos :type S%20Card%20Structure))
  ;[1 1 1] drag and drop des cartes
  (if (Variables|Default|Getis_my_turn)
    (Development|PrintString "On handle  le card drop")
    (bind _hitactor (CallFunction|GetMouseHitGrid))
    (if (.bSuccess (Utilities|Casting|CastToBP_Grid_cell _hitactor))
      (if (and (or (== (.cell_state (Variables|/Game/POW/game/grid/BP_Grid_cell.BP_Grid_cell_C|Getcell_info (.AsBP%20Grid%20Cell (Utilities|Casting|CastToBP_Grid_cell _hitactor)))) 0) (== (.cell_state (Variables|/Game/POW/game/grid/BP_Grid_cell.BP_Grid_cell_C|Getcell_info (.AsBP%20Grid%20Cell (Utilities|Casting|CastToBP_Grid_cell _hitactor)))) (+ (Variables|Default|Getplayer_number) 1))) (not (.is_taken (Variables|/Game/POW/game/grid/BP_Grid_cell.BP_Grid_cell_C|Getcell_info (.AsBP%20Grid%20Cell (Utilities|Casting|CastToBP_Grid_cell _hitactor))))))
        (CallFunction|CESERVERHandleCardDrop card_infos (.index (Variables|/Game/POW/game/grid/BP_Grid_cell.BP_Grid_cell_C|Getcell_info (.AsBP%20Grid%20Cell (Utilities|Casting|CastToBP_Grid_cell _hitactor))))))
      (else
        (Development|PrintString "pas grid cell")))))

(event Custom|CE_SERVER_handle_card_drop
  (params (card_infos :type S%20Card%20Structure) (cell_index :type Integer))
  (bind (_name _description _utility _damage _range _movement_ability _sp_abilities _life) (Utilities|Struct|BreakS_card card_infos))
  ;[1 1 1] drag and drop des cartes
  (if (Utilities|Enum|Equal(Enum) (.category (Utilities|Struct|BreakS_card card_infos)) "troups")
    (Development|PrintString "handle drop" true true "(R=1.000000,G=0.000000,B=0.060462,A=1.000000)" 5.0)
    (bind _returnvalue (Actor|GetActorOfClass "/Game/POW/game/grid/BP_Grid.BP_Grid_C"))
    (bind _grid_cell (Default|GetCellActorfromIndex _returnvalue cell_index))
    (if (and (or (== (.cell_state (Variables|/Game/POW/game/grid/BP_Grid_cell.BP_Grid_cell_C|Getcell_info _grid_cell)) 0) (== (.cell_state (Variables|/Game/POW/game/grid/BP_Grid_cell.BP_Grid_cell_C|Getcell_info _grid_cell)) (+ (Variables|Default|Getplayer_number) 1))) (not (.is_taken (Variables|/Game/POW/game/grid/BP_Grid_cell.BP_Grid_cell_C|Getcell_info _grid_cell))))
      (Default|CESERVERUpdateCell (.AsGS%20Arena (Utilities|Casting|CastToGS_arena (Game|GetGameState))) (Utilities|Struct|MakeCell (.index (Variables|/Game/POW/game/grid/BP_Grid_cell.BP_Grid_cell_C|Getcell_info _grid_cell)) (+ (Variables|Default|Getplayer_number) 1) true false))
      (bind _returnvalue_2 (Game|SpawnActorfromClass "/Game/POW/game/troup_actors/BP_TroupParent.BP_TroupParent_C" (Math|Transform|MakeTransform (Math|Vector|MakeVector (.x (Transformation|GetActorLocation _grid_cell)) (.y (Transformation|GetActorLocation _grid_cell)) (+ (.z (Transformation|GetActorLocation _grid_cell)) 5e+02)) (Math|Rotator|MakeRotator 0.0 0.0 (.yaw (Transformation|GetActorRotation (Game|Player|GetPlayerPawn (Variables|Default|Getplayer_number))))) "1,1,1") "Undefined" 0 (Variables|Default|Getplayer_number) (.index (Variables|/Game/POW/game/grid/BP_Grid_cell.BP_Grid_cell_C|Getcell_info _grid_cell)) false (Utilities|Struct|MakeTroupInfos (Utilities|String|StringToName _name) _description _damage _range _movement_ability 0 _life) 0))
      (Actor|SetOwner _returnvalue_2 self))))

(event Custom|CE_SERVER_MovePawnTo
  (params (Troup :type BP%20Troup%20Parent%20Object%20Reference) (target :type Integer))
  ;[1 1 1] Movement of the troup
  (Default|CESERVERMoveTroupto Troup target)
  (Variables|Default|Setselected_troup 0))

(event Custom|CE_display_notification
  (params (notificationText :type Text%20%28by%20ref%29))
  ;[1 1 1] display les différentes notifications
  (bind _returnvalue (UserInterface|CreateWidget "/Game/POW/game/UI/WI_notification.WI_notification_C" self notificationText))
  (bind _returnvalue_2 (Widget|Panel|AddChild (Variables|/Game/POW/game/UI/HUD_arena.HUD_arena_C|GetVB_notifications (Variables|Default|GetHUD_widget)) _returnvalue))
  (bind _asvertical_box_slot (Utilities|Casting|CastToVerticalBoxSlot _returnvalue_2)
    (:then
      (Layout|GridSlot|SetVerticalAlignment _asvertical_box_slot "VAlign_Top"))
    (:CastFailed
      (Development|PrintString "cast faillllllllllllllllll"))))

(event Custom|CE_C_BeginPlay
  ;[0.1538 1 0] begin play
  (Variables|Default|Settimer 0)
  (if (Pawn|IsLocalPlayerController)
    (bind _returnvalue (UserInterface|CreateWidget "/Game/POW/game/UI/HUD_arena.HUD_arena_C" self))
    (Variables|Default|SetHUD_widget _returnvalue)
    (UserInterface|Viewport|AddtoViewport _returnvalue 0)
    (CallFunction|OnGameStart-giveCards)))

(event Custom|CE_S_pass_turn
  ;[1 1 1] turn system
  (bind _asgm_arena (Utilities|Casting|CastToGM_arena (Game|GetGameMode)))
  (Default|CEChangeTurn _asgm_arena))

(event Custom|CE_create_terrain
  (params (terrain_to_add :type Integer))
  (bind _playerstate (Variables|GetPlayerState))
  (bind _asps_arena (Utilities|Casting|CastToPS_arena _playerstate))
  ;[1 1 1] input création terrain
  (Default|AddPendingTerrain _asps_arena terrain_to_add)
  (Networking|SwitchHasAuthority ; évite que le serveur fasse 2 fois la même chose
    (:Remote
      (Default|CESERVERAddTerrain _asps_arena terrain_to_add))))

(event Custom|CE_remove_terrain
  (params (terrain_to_remove :type Integer))
  (bind _playerstate (Variables|GetPlayerState))
  (bind _asps_arena (Utilities|Casting|CastToPS_arena _playerstate))
  ;[1 1 1] input destruction terrain
  (Default|AddPendingTerraintoRemove _asps_arena terrain_to_remove)
  (Networking|SwitchHasAuthority
    (:Remote
      (Default|CESERVERRemoveTerrain _asps_arena terrain_to_remove))))

(event Custom|CE_PC_undisplay_menu
  ;[1 1 1] toggle menu pause
  (Default|CEUndisplayMenu (Variables|Default|GetHUD_widget)))

(event Custom|CE_PC_display_menu
  ;[1 1 1] toggle menu pause
  (Default|CEDisplayMenu (Variables|Default|GetHUD_widget)))

(event Custom|CE_add_card_to_hand
  (params (card_infos :type S%20Card%20Structure))
  (bind _playerstate (Variables|GetPlayerState))
  (bind _asps_arena (Utilities|Casting|CastToPS_arena _playerstate))
  (bind _cards_in_hand (Variables|/Game/POW/game/PS_arena.PS_arena_C|Getcards_in_hand _asps_arena))
  (bind _returnvalue (Utilities|Array|Length _cards_in_hand))
  ;[1 1 1] ajoute une carte au deck avec animation
  (bind _returnvalue_2 (UserInterface|CreateWidget "/Game/POW/game/UI/WI_card.WI_card_C" (Game|GetPlayerController 0) card_infos (Variables|Default|Getanim_wi_card_to_hand)))
  (bind _returnvalue_3 (Widget|Panel|AddChild (Variables|/Game/POW/game/UI/HUD_arena.HUD_arena_C|GetCanvasPanel_HUD (Variables|Default|GetHUD_widget)) _returnvalue_2))
  (bind _ascanvas_panel_slot (Utilities|Casting|CastToCanvasPanelSlot _returnvalue_3))
  (Class|CanvasPanelSlot|SetZOrder _ascanvas_panel_slot 1)
  (bind _output_get (Variables|Default|SetCanvas_slot_new_card _ascanvas_panel_slot))
  (Class|CanvasPanelSlot|SetSize _output_get (Variables|Default|Getcard_size))
  (Variables|Default|Setstart_x (.x (Class|CanvasPanelSlot|GetPosition _output_get)))
  (Variables|Default|Setstart_y (.y (Class|CanvasPanelSlot|GetPosition _output_get)))
  (Math|Integer|IncrementInt (Variables|Default|Getnb_cards_in_hand)
    (:%20%20
      (bind _0_to_1 (Timeline|anim_wi_card_to_hand PlayFromStart)
        (:Update
          (Class|CanvasPanelSlot|SetPosition (Variables|Default|GetCanvas_slot_new_card) (Math|Vector2D|MakeVector2D (.x (Math|Vector|Lerp(Vector) (Math|Vector|MakeVector (Variables|Default|Getstart_x) (Variables|Default|Getstart_y) 0.0) (Math|Vector|MakeVector 0.0 0.0 0.0) _0_to_1)) (.y (Math|Vector|Lerp(Vector) (Math|Vector|MakeVector (Variables|Default|Getstart_x) (Variables|Default|Getstart_y) 0.0) (Math|Vector|MakeVector 0.0 0.0 0.0) _0_to_1))))
          (Class|CanvasPanelSlot|SetAnchors (Variables|Default|GetCanvas_slot_new_card) (Utilities|Struct|MakeAnchors (Math|Vector2D|MakeVector2D (.x (Math|Vector|Lerp(Vector) (Math|Vector|MakeVector 0.5 1.0 0.0) (Math|Vector|MakeVector 0.5 0.8 0.0) _0_to_1)) (.y (Math|Vector|Lerp(Vector) (Math|Vector|MakeVector 0.5 1.0 0.0) (Math|Vector|MakeVector 0.5 0.8 0.0) _0_to_1))) (Math|Vector2D|MakeVector2D (.x (Math|Vector|Lerp(Vector) (Math|Vector|MakeVector 0.5 1.0 0.0) (Math|Vector|MakeVector 0.5 0.8 0.0) _0_to_1)) (.y (Math|Vector|Lerp(Vector) (Math|Vector|MakeVector 0.5 1.0 0.0) (Math|Vector|MakeVector 0.5 0.8 0.0) _0_to_1)))))
          (Class|CanvasPanelSlot|SetAlignment (Variables|Default|GetCanvas_slot_new_card) (Math|Vector2D|MakeVector2D (.x (Math|Vector|Lerp(Vector) (Math|Vector|MakeVector 0.0 0.0 0.0) (Math|Vector|MakeVector (- (Math|Conversions|ToFloat(Integer) (- (Variables|Default|Getnb_cards_in_hand) (/ _returnvalue 2))) (* (Math|Integer|%(Integer) _returnvalue 2) 0.5)) 0.0 0.0) _0_to_1)) (.y (Math|Vector|Lerp(Vector) (Math|Vector|MakeVector 0.0 0.0 0.0) (Math|Vector|MakeVector (- (Math|Conversions|ToFloat(Integer) (- (Variables|Default|Getnb_cards_in_hand) (/ _returnvalue 2))) (* (Math|Integer|%(Integer) _returnvalue 2) 0.5)) 0.0 0.0) _0_to_1)))))
        (:Finished
          (Variables|Default|SetCanvas_slot_pause_menu 0))))))

(event Custom|OnGameStart-give_cards
  ;[1 1 1] distribue les cartes (5) pour le début de partie
  (bind _arrayelement (Utilities|ForEachLoopwithDelay (Variables|/Game/POW/game/PS_arena.PS_arena_C|Getcards_in_hand (.AsPS%20Arena (Utilities|Casting|CastToPS_arena (Variables|GetPlayerState)))) 0.31)
    (:LoopBody
      (Development|PrintString (.name (Utilities|Struct|BreakS_card _arrayelement)))
      (CallFunction|CEAddCardtoHand _arrayelement))))

(event Input|KeyboardEvents|T
  (params (Key :type Key%20Structure :default "None"))
  ;[1 0 0] test path finding
  (:Pressed
    (bind _hitactor (CallFunction|GetMouseHitGrid))
    (bind _asbp_grid_cell (Utilities|Casting|CastToBP_Grid_cell _hitactor))
    (Default|TESTPathFinding _asbp_grid_cell)))

(event Input|KeyboardEvents|C
  (params (Key :type Key%20Structure :default "None"))
  ;[1 0.1172 0.1172] debug
  (:Pressed
    (for _array_element (Variables|/Game/POW/game/PS_arena.PS_arena_C|Getplayer_cards (.AsPS%20Arena (Utilities|Casting|CastToPS_arena (Variables|GetPlayerState))))
      (Development|PrintString (.name _array_element)))))

(event Input|KeyboardEvents|E
  (params (Key :type Key%20Structure :default "None"))
  ;[1 0 0.03055] debug pour voir combien de terrain possède chaque joueur
  (:Pressed
    (Development|PrintString (Utilities|String|Append (Utilities|String|ToString(Integer) (Utilities|Array|Length (Variables|/Game/POW/game/GS_arena.GS_arena_C|Getcells_placed_array (.AsGS%20Arena (Utilities|Casting|CastToGS_arena (Game|GetGameState)))))) " terrains ont été placés"))))

(event Input|MouseEvents|LeftMouseButton
  (params (Key :type Key%20Structure :default "None"))
  (bind _hitresult (Game|Player|GetHitResultUnderCursorbyChannel "TraceTypeQuery2" false))
  (bind _hitactor (Collision|BreakHitResult _hitresult))
  ;[1 1 1] left-right clicks handle
  (:Pressed
    (if (Variables|Default|Getis_my_turn)
      (bind _asbp_troup_parent (Utilities|Casting|CastToBP_TroupParent _hitactor)
        (:then
          (Development|PrintString "on clique dessus")
          (if (== (Variables|/Game/POW/game/troup_actors/BP_TroupParent.BP_TroupParent_C|Getowner_index _asbp_troup_parent) (Variables|Default|Getplayer_number))
            (Variables|Default|Setselected_troup _asbp_troup_parent)
            (Development|PrintString "on le selectionne")
            (else
              (bind _returnvalue (Class|TroupParent|Attack (Variables|Default|Getselected_troup) _asbp_troup_parent))
              (Development|PrintString "attaque")
              (Development|PrintString (Utilities|String|ToString(Boolean) _returnvalue)))))
        (:CastFailed
          (bind _asbp_grid_cell (Utilities|Casting|CastToBP_Grid_cell _hitactor)
            (:then
              (if (Utilities|IsValid (Variables|Default|Getselected_troup))
                (Development|PrintString "on bouge")
                (if (and (not (.is_taken (Variables|/Game/POW/game/grid/BP_Grid_cell.BP_Grid_cell_C|Getcell_info _asbp_grid_cell))) (Math|Boolean|Equal(Boolean) (.is_walkable (Variables|/Game/POW/game/grid/BP_Grid_cell.BP_Grid_cell_C|Getcell_info _asbp_grid_cell)) true))
                  (bind _returnvalue_2 (Actor|GetActorOfClass "/Game/POW/game/grid/BP_Grid.BP_Grid_C"))
                  (Default|CEUnshowPath _returnvalue_2)
                  (CallFunction|CESERVERMovePawnto (Variables|Default|Getselected_troup) (.index (Variables|/Game/POW/game/grid/BP_Grid_cell.BP_Grid_cell_C|Getcell_info _asbp_grid_cell)))
                  (Variables|Default|Setselected_troup 0)
                  (else
                    (Variables|Default|Setselected_troup 0)))
                (else
                  (Development|PrintString "selected pawn pas valide"))))
            (:CastFailed
              (Variables|Default|Setselected_troup 0)))))
      (else
        (bind _asbp_grid_cell_2 (Utilities|Casting|CastToBP_Grid_cell _hitactor))
        (Default|CECellLeftClicked _asbp_grid_cell_2)))))

(event Input|MouseEvents|RightMouseButton
  (params (Key :type Key%20Structure :default "None"))
  ;[1 1 1] left-right clicks handle
  (:Pressed
    (if (not (Variables|Default|Getis_my_turn))
      (bind _asbp_grid_cell (Utilities|Casting|CastToBP_Grid_cell (.HitActor (Collision|BreakHitResult (.HitResult (Game|Player|GetHitResultUnderCursorbyChannel "TraceTypeQuery2" false))))))
      (Default|CECellRightClicked _asbp_grid_cell))))

(event Input|KeyboardEvents|Escape
  (params (Key :type Key%20Structure :default "None"))
  ;[1 1 1] toggle menu pause
  (:Pressed
    (if (== (Variables|/Game/POW/game/UI/HUD_arena.HUD_arena_C|Getwi_pause_menu (Variables|Default|GetHUD_widget)) 0)
      (CallFunction|CEPCDisplayMenu)
      (else
        (CallFunction|CEPCUndisplayMenu)))))

(event Input|KeyboardEvents|Y
  (params (Key :type Key%20Structure :default "None"))
  (bind _returnvalue (Game|GetGameState))
  (bind _asgs_arena (Utilities|Casting|CastToGS_arena _returnvalue))
  ;[1 0 0] get nb de cases possédées par les 2 joueurs
  (:Pressed
    (Development|PrintString (Utilities|String|ToString(Text) (Utilities|Text|FormatText "Le player 1 possède {p1_cases} cases\\n le player 2 possède {p2_cases} cases" (Utilities|Array|Length (Variables|/Game/POW/game/GS_arena.GS_arena_C|Getplayer1_possessed_cells _asgs_arena)) (Utilities|Array|Length (Variables|/Game/POW/game/GS_arena.GS_arena_C|Getplayer2_possessed_cells _asgs_arena)))))))

(fn ConstructionScript)

(fn SetMyTurn
  (params (is_my_turn? :type Boolean))
  (bind _output_get (Variables|Default|Setis_my_turn is_my_turn?))
  (Default|CallOnMyTurnChanged _output_get))

(fn GetMouseHitGrid
  (bind _returnvalue (Class|WidgetLayoutLibrary|GetMousePositiononViewport))
  (bind _outhit (Collision|LineTraceByChannel (.WorldPosition (Class|GameplayStatics|DeprojectScreentoWorld self (* _returnvalue (Class|WidgetLayoutLibrary|GetViewportScale)))) (+ (.WorldPosition (Class|GameplayStatics|DeprojectScreentoWorld self (* _returnvalue (Class|WidgetLayoutLibrary|GetViewportScale)))) (* (.WorldDirection (Class|GameplayStatics|DeprojectScreentoWorld self (* _returnvalue (Class|WidgetLayoutLibrary|GetViewportScale)))) 8e+03)) "TraceTypeQuery2" false 0 "ForDuration"))
  (return (.hitactor _outhit)))