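; Arena game mode that runs match setup and turn order for a two-player card game.
; It collects joining controllers and starts once the session count is met, or at two players if the session lookup fails.
; Startup spawns card pawns, fills hands from each PlayerState's saved cards, then picks a random first player.
; Turn changes toggle a player index, notify both PC_arena controllers and have GS_arena update the terrain.
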(event Custom|CE_give_player_cards
  ;[1 1 1] set les cartes au début du jeu (au hasard)
  (for _array_element (Variables|Default|Getplayer_controllers)
    (bind _asps_arena (Utilities|Casting|CastToPS_arena (Variables|/Script/Engine.Controller|GetPlayerState _array_element)))
    (Default|CESERVERLoadSavedData _asps_arena)
    (for _index (range 0 (Variables|Default|Getstart_player_cards))
      (Utilities|Array|Add (Variables|/Game/POW/game/PS_arena.PS_arena_C|Getcards_in_hand _asps_arena) (Utilities|Array|Get(acopy) (Variables|/Game/POW/game/PS_arena.PS_arena_C|Getplayer_cards _asps_arena) _index)))))

(event Custom|CE_start_game
  ;[0 1 0.07082] start game
  (CallFunction|CESetPlayerPawn)
  (CallFunction|CEGivePlayerCards)
  (Utilities|FlowControl|Delay 2.0)
  (for (_array_element _array_index) (Variables|Default|Getplayer_controllers)
    (Variables|/Game/POW/game/PC_arena.PC_arena_C|Setplayer_number (.AsPC%20Arena (Utilities|Casting|CastToPC_arena _array_element)) _array_index)
    (Default|CECBeginPlay (.AsPC%20Arena (Utilities|Casting|CastToPC_arena _array_element))))
  (CallFunction|CESetPlayersTurn))

(event Custom|CE_set_player_pawn
  ;[1 1 1] set player pawn
  (for (_array_element _array_index) (Variables|Default|Getplayer_controllers)
    (bind _returnvalue (Game|SpawnActorfromClass "/Game/POW/game/player_cards_pawn.Player_cards_pawn_C" (Transformation|GetActorTransform (Class|GameModeBase|FindPlayerStart _array_element (Utilities|String|ToString(Integer) _array_index))) "Undefined" 0 0))
    (Pawn|Possess _array_element _returnvalue)))

(event Custom|CE_set_players_turn
  (bind _returnvalue (Math|Random|RandomInteger 2))
  ;[1 1 1] set players turn au hasard (appelé au début de partie)
  (Variables|Default|Setcurrent_player_turn _returnvalue)
  ;;[1 0.01675 0] juste pour être sûr 0-1
  (Development|PrintString (Utilities|String|ToString(Integer) _returnvalue))
  (bind _player_controller (CallFunction|GetPlayerinTurn))
  (Default|CECStartTurn _player_controller)
  (bind _player_controller_2 (CallFunction|GetPlayerNotinTurn))
  (Default|CECEndTurn _player_controller_2))

(event Custom|CE_change_turn
  ;[1 1 1] change turn
  (bind _player_controller (CallFunction|GetPlayerinTurn))
  (Default|CECEndTurn _player_controller)
  (Variables|Default|Setcurrent_player_turn (select (== (Variables|Default|Getcurrent_player_turn) 0) 1 0))
  (bind _player_controller_2 (CallFunction|GetPlayerinTurn))
  (Default|CECStartTurn _player_controller_2)
  (CallFunction|CEUpdateTurnInfos))

(event Custom|CE_update_turn_infos
  (bind _asgs_arena (Utilities|Casting|CastToGS_arena (Game|GetGameState)))
  (Default|CESUpdateTerrain _asgs_arena))

(event EventHandleStartingNewPlayer
  (params (NewPlayer :type Player%20Controller%20Object%20Reference))
  (bind _player_controllers (Variables|Default|Getplayer_controllers))
  (bind _returnvalue (Utilities|Array|Length _player_controllers))
  ;[1 1 1] event new player
  (Utilities|Array|AddUnique _player_controllers NewPlayer)
  (bind _numconnections (Class|AdvancedSessionsLibrary|GetSessionSettings)
    (:OnSuccess
      (if (== _numconnections _returnvalue)
        (Development|PrintString "on peut commencer" :!label _label)
        (CallFunction|CEStartGame)))
    (:OnFailure
      ;;[1 0.8085 0.09327] tant qu'on est en listen server
      (if (== 2 _returnvalue)
        (goto _label)))))

(fn ConstructionScript)

(fn GetPlayerinTurn
  (return (.AsPC%20Arena (Utilities|Casting|CastToPC_arena (Game|GetPlayerController (Variables|Default|Getcurrent_player_turn))))))

(fn GetPlayerNotinTurn
  (return (.AsPC%20Arena (Utilities|Casting|CastToPC_arena (Game|GetPlayerController (select (== (Variables|Default|Getcurrent_player_turn) 0) 1 0))))))