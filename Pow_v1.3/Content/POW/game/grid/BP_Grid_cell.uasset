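; BP_Grid_cell is one tile of the arena grid, with visibility and material driven by its cell_state.
; On the player's turn, hovering asks BP_Grid to show or clear the path from the selected owned troop.
; Otherwise, hovering highlights the tile, or with a mouse button held paints or erases terrain through PC_arena, updating cell_state.
; A debug event tests FindPath with a hardcoded start and briefly colours the resulting path.
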(event OnBeginCursorOver(tileStaticMesh)
  (params (TouchedComponent :type Primitive%20Component%20Object%20Reference))
  (bind _returnvalue (Game|GetPlayerController 0))
  ;[1 1 1] cell begin hover
  (bind _aspc_arena (Utilities|Casting|CastToPC_arena _returnvalue))
  (if (Variables|/Game/POW/game/PC_arena.PC_arena_C|Getis_my_turn _aspc_arena)
    (CallFunction|CECellinPath)
    (elif (Game|Player|IsInputKeyDown _returnvalue "LeftMouseButton")
      (CallFunction|CECellLeftClicked)
      (elif (Game|Player|IsInputKeyDown _returnvalue "RightMouseButton")
        (CallFunction|CECellRightClicked)
        (else
          (Rendering|Material|SetMaterial (Variables|Default|GettileStaticMesh) 0 "/Game/MSPresets/MS_DefaultMaterial/MS_DefaultMaterial.MS_DefaultMaterial")
          (Rendering|SetVisibility (Variables|Default|GettileStaticMesh) true false)
          (Development|PrintString (Utilities|String|ToString(Integer) (.index (Variables|Default|Getcell_info)))))))))

(event OnEndCursorOver(tileStaticMesh)
  (params (TouchedComponent :type Primitive%20Component%20Object%20Reference))
  ;[1 1 1] cell end hover
  (bind _aspc_arena (Utilities|Casting|CastToPC_arena (Game|GetPlayerController 0)))
  (if (Variables|/Game/POW/game/PC_arena.PC_arena_C|Getis_my_turn _aspc_arena)
    (CallFunction|CENotCellinPath)
    (else
      (CallFunction|CERefreshMaterial))))

(event Custom|CE_cell_left_clicked
  ;[1 1 1] cell_clicked
  (if (== (.cell_state (Variables|Default|Getcell_info)) -1)
    (Default|CECreateTerrain (.AsPC%20Arena (Utilities|Casting|CastToPC_arena (Game|GetPlayerController 0))) (.index (Variables|Default|Getcell_info)))
    (Rendering|Material|SetMaterial (Variables|Default|GettileStaticMesh) 0 "/Game/Geometry/Meshes/CubeMaterial.CubeMaterial")
    (Rendering|SetVisibility (Variables|Default|GettileStaticMesh) true false)
    (Variables|Default|Setcell_info (Utilities|Struct|MakeCell (.index (Variables|Default|Getcell_info)) 3 (.is_taken (Variables|Default|Getcell_info)) (.is_walkable (Variables|Default|Getcell_info))))))

(event Custom|CE_cell_right_clicked
  ;[1 1 1] cell_clicked
  (if (== (.cell_state (Variables|Default|Getcell_info)) 3)
    (Default|CERemoveTerrain (.AsPC%20Arena (Utilities|Casting|CastToPC_arena (Game|GetPlayerController 0))) (.index (Variables|Default|Getcell_info)))
    (Rendering|SetVisibility (Variables|Default|GettileStaticMesh) false false)
    (Variables|Default|Setcell_info (Utilities|Struct|MakeCell (.index (Variables|Default|Getcell_info)) -1 (.is_taken (Variables|Default|Getcell_info)) (.is_walkable (Variables|Default|Getcell_info))))))

(event Custom|TEST_path_finding
  (bind _tmp_cells_info (Variables|Default|Gettmp_cells_info))
  (bind _returnvalue (Actor|GetActorOfClass "/Game/POW/game/grid/BP_Grid.BP_Grid_C"))
  (for _array_element (Variables|/Game/POW/game/grid/BP_Grid.BP_Grid_C|Getcells_array _returnvalue)
    ;[1 1 1] debug
    (Utilities|Array|AddUnique (Variables|Default|Gettmp_cells_info) (Variables|BP_Grid_cell_C|Getcell_info _array_element)))
  (Development|PrintString (Utilities|String|ToString(Integer) (Utilities|Array|Length _tmp_cells_info)))
  (bind _returnvalue_2 (Class|PathFinding|FindPath 28 23 380 (.index (Variables|Default|Getcell_info)) _tmp_cells_info false))
  (for _array_element_2 _returnvalue_2
    (Development|PrintString (Utilities|String|ToString(Integer) _array_element_2))
    (Rendering|Material|SetMaterial (Variables|BP_Grid_cell_C|GettileStaticMesh (Utilities|Array|Get(acopy) (Variables|/Game/POW/game/grid/BP_Grid.BP_Grid_C|Getcells_array _returnvalue) _array_element_2)) 0 "/Game/Mannequin/Character/Materials/M_Male_Body.M_Male_Body"))
  (Utilities|FlowControl|Delay 2.0)
  (for _array_element_3 _returnvalue_2
    (CallFunction|CERefreshMaterial (Utilities|Array|Get(acopy) (Variables|/Game/POW/game/grid/BP_Grid.BP_Grid_C|Getcells_array _returnvalue) _array_element_3))))

(event Custom|CE_refresh_material
  (bind _tilestaticmesh (Variables|Default|GettileStaticMesh))
  ;[1 1 1] refresh le material en fonction du cell_state
  (switch int (+ (.cell_state (Variables|Default|Getcell_info)) 1)
    (:0
      (Rendering|SetVisibility _tilestaticmesh false false))
    (:1
      (Rendering|SetVisibility _tilestaticmesh true false)
      (Rendering|Material|SetMaterial _tilestaticmesh 0 "/Game/Megascans/3D_Assets/Roman_Stone_Floor_tkkrcayfa/Roman_Stone_Floor_tkkrcayfa_inst.Roman_Stone_Floor_tkkrcayfa_inst"))
    (:2
      (Rendering|SetVisibility _tilestaticmesh true false)
      (Rendering|Material|SetMaterial _tilestaticmesh 0 "/Game/Mannequin/Character/Materials/M_Male_Body.M_Male_Body"))
    (:3
      (Rendering|SetVisibility _tilestaticmesh true false)
      (Rendering|Material|SetMaterial _tilestaticmesh 0 "/Game/Mannequin/Character/Materials/MI_Female_Body.MI_Female_Body"))
    (:4
      (Rendering|SetVisibility _tilestaticmesh true false)
      (Rendering|Material|SetMaterial _tilestaticmesh 0 "/Game/Geometry/Meshes/CubeMaterial.CubeMaterial"))))

(event Custom|CE_C_refresh_cell
  ;[1 1 1] refresh the cell
  (CallFunction|CERefreshMaterial))

(event Custom|CE_cell_in_path
  (bind _returnvalue (Game|GetPlayerController 0))
  (bind _cell_info (Variables|Default|Getcell_info))
  (bind _aspc_arena (Utilities|Casting|CastToPC_arena _returnvalue))
  (bind _selected_troup (Variables|/Game/POW/game/PC_arena.PC_arena_C|Getselected_troup _aspc_arena))
  ;[1 1 1] appelle le grid pour mettre en surbrillance les cells sur le chemin
  (if (Math|Boolean|ANDBoolean (== (Variables|/Game/POW/game/troup_actors/BP_TroupParent.BP_TroupParent_C|Getowner_index _selected_troup) (Variables|/Game/POW/game/PC_arena.PC_arena_C|Getplayer_number _aspc_arena)) (!= (.cell_state _cell_info) -1) (!= (.cell_state _cell_info) 3))
    (bind _returnvalue_2 (Actor|GetActorOfClass "/Game/POW/game/grid/BP_Grid.BP_Grid_C"))
    (Default|CEShowPath _returnvalue_2 (Variables|/Game/POW/game/troup_actors/BP_TroupParent.BP_TroupParent_C|Getposition_in_grid _selected_troup) (.index (Variables|Default|Getcell_info)) (Variables|/Game/POW/game/troup_actors/BP_TroupParent.BP_TroupParent_C|Getdiag_movement? _selected_troup))))

(event Custom|CE_not_cell_in_path
  ;[1 1 1] appelle le grid pour enlever la surbrillance du chemin
  (bind _returnvalue (Actor|GetActorOfClass "/Game/POW/game/grid/BP_Grid.BP_Grid_C"))
  (Default|CEUnshowPath _returnvalue))

(fn ConstructionScript)