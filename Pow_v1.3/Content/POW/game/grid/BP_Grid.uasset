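; BP_Grid is the game's grid actor: on BeginPlay it spawns a Rows by Columns set of initially invisible BP_Grid_cell actors, owned by player controller 0.
; Cells live in a flat row-major array, and Update copies incoming cell infos into them and refreshes each one.
; Path preview passes those infos to FindPath, highlights the returned cells with a material, and later restores them from the stored indices.
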(event Custom|CE_showPath
  (params (start :type Integer) (target :type Integer) (allow_diag_path :type Boolean))
  ;[1 1 1] mets en surbrillance le chemin estimé
  (bind _cells_infos_array (CallFunction|MakeCellsInfosArray))
  (bind _returnvalue (Class|PathFinding|FindPath (Variables|Default|Getrows) (Variables|Default|Getcolumns) start target _cells_infos_array allow_diag_path))
  (Variables|Default|Seton_path_cells_index _returnvalue)
  (for _array_element _returnvalue
    (Rendering|Material|SetMaterial (Variables|/Game/POW/game/grid/BP_Grid_cell.BP_Grid_cell_C|GettileStaticMesh (Utilities|Array|Get(acopy) (Variables|Default|Getcells_array) _array_element)) 0 "/Game/Geometry/Meshes/CubeMaterial.CubeMaterial")))

(event Custom|CE_unshowPath
  (bind _on_path_cells_index (Variables|Default|Geton_path_cells_index))
  ;[1 1 1] enlève la surbrillance
  (for _array_element _on_path_cells_index
    (Default|CERefreshMaterial (Utilities|Array|Get(acopy) (Variables|Default|Getcells_array) _array_element)))
  (Utilities|Array|Clear _on_path_cells_index))

(event EventBeginPlay
  (bind _defaultsceneroot (Variables|Default|GetDefaultSceneRoot))
  (bind _returnvalue (Transformation|GetWorldTransform _defaultsceneroot))
  ;[1 1 1] begin play - spawn toutes les cases
  (Actor|SetOwner (Game|GetPlayerController 0))
  (for _index (range 0 (- (Variables|Default|Getrows) 1))
    (for _index_2 (range 0 (- (Variables|Default|Getcolumns) 1))
      (bind _returnvalue_2 (Game|SpawnActorfromClass "/Game/POW/game/grid/BP_Grid_cell.BP_Grid_cell_C" (Math|Transform|MakeTransform (+ (Math|Vector|MakeVector (+ (* _index (Variables|Default|Getcell_size)) (/ (Variables|Default|Getcell_size) 2.0)) (+ (* _index_2 (Variables|Default|Getcell_size)) (/ (Variables|Default|Getcell_size) 2.0)) 0.0) (.location _returnvalue)) (.rotation _returnvalue) "0.040000,0.040000,0.040000") "AlwaysSpawn" 0 (Utilities|Struct|MakeCell (+ (* _index (Variables|Default|Getcolumns)) _index_2) -1 false false) 0))
      (Actor|SetOwner _returnvalue_2 (Game|GetPlayerController 0))
      (Rendering|SetVisibility (Variables|/Game/POW/game/grid/BP_Grid_cell.BP_Grid_cell_C|GettileStaticMesh _returnvalue_2) false false)
      (Utilities|Array|Add (Variables|Default|Getcells_array) _returnvalue_2))))

(fn ConstructionScript)

(fn GetCellActorfromIndex
  (params (cell_index :type Integer))
  (return (Utilities|Array|Get(acopy) (Variables|Default|Getcells_array) cell_index)))

(fn Update
  (params (new_cells_infos :type Array%20of%20Cell%20Structures))
  (for _array_element new_cells_infos
    (Variables|/Game/POW/game/grid/BP_Grid_cell.BP_Grid_cell_C|Setcell_info (Utilities|Array|Get(acopy) (Variables|Default|Getcells_array) (.index _array_element)) (Utilities|Struct|MakeCell (.index _array_element) (.cell_state _array_element) (.is_taken _array_element) (.is_walkable _array_element)))
    (Development|PrintString (Utilities|String|ToString(Integer) (.index _array_element)))
    (Default|CECRefreshCell (Utilities|Array|Get(acopy) (Variables|Default|Getcells_array) (.index _array_element)))))

(fn MakeCellsInfosArray
  (for _array_element (Variables|Default|Getcells_array)
    (Utilities|Array|Add (LocalVariables|Getlocal_card_array) (Variables|/Game/POW/game/grid/BP_Grid_cell.BP_Grid_cell_C|Getcell_info _array_element)))
  (return (LocalVariables|Getlocal_card_array)))